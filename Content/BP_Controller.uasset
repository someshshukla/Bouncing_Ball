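; BP_Controller is a player controller that rolls or pushes the controlled BP_Player's physics Sphere around with keyboard and mouse.
; Each tick it polls WASD and applies mass-independent force along the Camera's forward and right vectors, while mouse axes feed yaw and inverted pitch input.
; Space applies an upward velocity-change impulse when CanJump is true, then clears the flag, which this file never sets back.
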(event EventBeginPlay
  (bind _asbp_player (Utilities|Casting|CastToBP_Player (Pawn|GetControlledPawn)))
  (Variables|Default|SetBP%20Player _asbp_player))

(event EventTick
  (params (DeltaSeconds :type Float%20%28single-precision%29))
  (bind _bp_player (Variables|Default|GetBP%20Player))
  (bind _bp_player_2 (Variables|Default|GetBP%20Player))
  (bind _bp_player_3 (Variables|Default|GetBP%20Player))
  (bind _bp_player_4 (Variables|Default|GetBP%20Player))
  (Utilities|FlowControl|Sequence
    (:then_0
      ;[1 1 1] W
      (if (Game|Player|IsInputKeyDown "W")
        (Physics|AddForce (Variables|/Game/BP_Player.BP_Player_C|GetSphere _bp_player_2) (* (Math|Vector|GetForwardVector (Variables|/Game/BP_Player.BP_Player_C|GetCamera _bp_player_2)) 1e+03) "None" true)))
    (:then_1
      ;[1 1 1] S
      (if (Game|Player|IsInputKeyDown "S")
        (Physics|AddForce (Variables|/Game/BP_Player.BP_Player_C|GetSphere _bp_player_3) (* (Math|Vector|GetForwardVector (Variables|/Game/BP_Player.BP_Player_C|GetCamera _bp_player_3)) -1e+03) "None" true)))
    (:then_2
      ;[1 1 1] A
      (if (Game|Player|IsInputKeyDown "A")
        (Physics|AddForce (Variables|/Game/BP_Player.BP_Player_C|GetSphere _bp_player_4) (* (Math|Vector|GetRightVector (Variables|/Game/BP_Player.BP_Player_C|GetCamera _bp_player_4)) -1e+03) "None" true)))
    (:then_3
      ;[1 1 1] D
      (if (Game|Player|IsInputKeyDown "D")
        (Physics|AddForce (Variables|/Game/BP_Player.BP_Player_C|GetSphere _bp_player) (* (Math|Vector|GetRightVector (Variables|/Game/BP_Player.BP_Player_C|GetCamera _bp_player)) 1e+03) "None" true)))))

(event Input|MouseEvents|MouseX
  (params (AxisValue :type Float%20%28single-precision%29))
  ;[1 1 1] Mouse control
  (Class|PlayerController|AddYawInput AxisValue))

(event Input|MouseEvents|MouseY
  (params (AxisValue :type Float%20%28single-precision%29))
  ;[1 1 1] Mouse control
  (Class|PlayerController|AddPitchInput (* AxisValue -1.0)))

(event Input|KeyboardEvents|SpaceBar
  (params (Key :type Key%20Structure :default "None"))
  ;[1 1 1] SpaceJump
  (:Pressed
    (if (Variables|Default|GetcanJump)
      (Variables|Default|SetcanJump false)
      (Physics|AddImpulse (Variables|/Game/BP_Player.BP_Player_C|GetSphere (Variables|Default|GetBP%20Player)) "0.000000,0.000000,1000.000000" "None" true))))

(fn ConstructionScript)